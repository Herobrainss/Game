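; Unit that works through a queue of orders stored as parallel Actions and Positions arrays, seeded on BeginPlay with a hard-coded Move.
; DoAction dispatches the current action by name; Move uses SimpleMoveToLocation, while Move Hold Contact is an empty stub.
; Tick sets yaw from the previous-minus-current location vector, then advances to the next action when near the target.
; An unconnected synchronous pathfinding variant remains in Move.
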(event EventBeginPlay
  (Variables|Default|SetLastLocation (Transformation|GetActorLocation))
  (CallFunction|AddDefaultTarget)
  (CallFunction|DoAction))

(event EventActorBeginOverlap
  (params (OtherActor :type Actor%20Object%20Reference)))

(event EventTick
  (params (DeltaSeconds :type Float%20%28single-precision%29))
  (bind _returnvalue (Transformation|GetActorLocation))
  ;[1 1 1] SetRotation
  (Transformation|SetActorRotation (Math|Rotator|MakeRotator 0.0 0.0 (.Yaw (Math|Vector|GetYawPitchfromVector (- (Variables|Default|GetLastLocation) _returnvalue)))))
  (bind _output_get (Variables|Default|SetLastLocation _returnvalue))
  (bind _length (CallFunction|GetLength))
  (if (< (Variables|Default|GetActionIndex) _length)
    (if (< (Math|Vector|VectorLength (- _output_get (Utilities|Array|Get(acopy) (Variables|Default|GetPositions) (Variables|Default|GetActionIndex)))) 5e+01)
      (Math|Integer|IncrementInt (Variables|Default|GetActionIndex)
        (:%20%20
          (CallFunction|DoAction))))))

(fn ConstructionScript)

(fn IndexinBounds
  (return (and (< (Utilities|Array|Length (Variables|Default|GetActions)) (Variables|Default|GetActionIndex)) (< (Utilities|Array|Length (Variables|Default|GetPositions)) (Variables|Default|GetActionIndex)))))

(fn Move
  (params (Target%20Location :type Vector))
  ;[1 1 1] Working Move
  (AI|Navigation|SimpleMovetoLocation (Pawn|GetController self) Target%20Location)
  (return true))

(fn GetPosition
  (return (Utilities|Array|Get(acopy) (Variables|Default|GetPositions) (Variables|Default|GetActionIndex))))

(fn GetAction
  (return (Utilities|Array|Get(acopy) (Variables|Default|GetActions) (Variables|Default|GetActionIndex))))

(fn GetLength
  (return (Utilities|Array|Length (Variables|Default|GetPositions))))

(fn AddDefaultTarget
  (Utilities|Array|Add (Variables|Default|GetPositions) "1800.000000,1000.000000,550.000000")
  (Utilities|Array|Add (Variables|Default|GetActions) "Move")
  (if (and (> (Utilities|Array|Length (Variables|Default|GetPositions)) 0) (> (Utilities|Array|Length (Variables|Default|GetActions)) 0))
    _
    (else
      (Class|VisualLoggerKismetLibrary|LogText "Unit is missing location and/or action array" "Blueprint Log")))
  (return))

(fn DoAction
  (bind _action (CallFunction|GetAction))
  (switch string _action
    (:Default
      _)
    (:Move
      (bind _item (CallFunction|GetPosition))
      (CallFunction|Move self _item))
    (:MoveHoldContact
      _))
  (return))